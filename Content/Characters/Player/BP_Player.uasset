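; Player character for a Pac-Man-style game, steered along linked control points with queued turns, instant reversals and mask-dependent paths.
; Overlaps collect pellets, unlock colored masks via gameplay tags, cost a life on enemies with different masks, and kill vulnerable enemies.
; Power pellets make all enemies vulnerable until a delay resets DamageState.
; It also creates the score widget and toggles pause; mask-equip inputs and death only print messages.
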(event Custom|DesiredDirectionChanged
  (if (Utilities|Enum|Equal(Enum) (Variables|Default|GetDesiredDirection) (CallFunction|GetOppositeDirection (Variables|Default|GetCurrentDirection)))
    (CallFunction|TurnAround)))

(event Input|EnhancedActionEvents|EnhancedInputActionIA_Move_Up
  (params (ActionValue :type Float%20%28double-precision%29) (ElapsedSeconds :type Float%20%28double-precision%29) (TriggeredSeconds :type Float%20%28double-precision%29) (InputAction :type Input%20Action%20Object%20Reference :default "/Game/Characters/Player/IA_Move_Up.IA_Move_Up"))
  ;[0.15 0 0.08376 0.5] Input Logic
  (:Started
    (Variables|Default|SetDesiredDirection (select (> ActionValue 0.0) "NewEnumerator0" "NewEnumerator1"))
    (CallFunction|DesiredDirectionChanged)))

(event Input|EnhancedActionEvents|EnhancedInputActionIA_Move_Right
  (params (ActionValue :type Float%20%28double-precision%29) (ElapsedSeconds :type Float%20%28double-precision%29) (TriggeredSeconds :type Float%20%28double-precision%29) (InputAction :type Input%20Action%20Object%20Reference :default "/Game/Characters/Player/IA_Move_Right.IA_Move_Right"))
  ;[0.15 0 0.08376 0.5] Input Logic
  (:Started
    (Variables|Default|SetDesiredDirection (select (> ActionValue 0.0) "NewEnumerator3" "NewEnumerator2"))
    (CallFunction|DesiredDirectionChanged)))

(event Input|EnhancedActionEvents|EnhancedInputActionIA_Mask_1
  (params (ActionValue :type Boolean) (ElapsedSeconds :type Float%20%28double-precision%29) (TriggeredSeconds :type Float%20%28double-precision%29) (InputAction :type Input%20Action%20Object%20Reference :default "/Game/Characters/Player/IA_Mask_1.IA_Mask_1"))
  ;[0.15 0 0.08376 0.5] Input Logic
  (Development|PrintString "Mask 1 Equipped"))

(event Input|EnhancedActionEvents|EnhancedInputActionIA_Mask_2
  (params (ActionValue :type Boolean) (ElapsedSeconds :type Float%20%28double-precision%29) (TriggeredSeconds :type Float%20%28double-precision%29) (InputAction :type Input%20Action%20Object%20Reference :default "/Game/Characters/Player/IA_Mask_2.IA_Mask_2"))
  ;[0.15 0 0.08376 0.5] Input Logic
  (Development|PrintString "Mask 2 Equipped"))

(event Input|EnhancedActionEvents|EnhancedInputActionIA_Mask_3
  (params (ActionValue :type Boolean) (ElapsedSeconds :type Float%20%28double-precision%29) (TriggeredSeconds :type Float%20%28double-precision%29) (InputAction :type Input%20Action%20Object%20Reference :default "/Game/Characters/Player/IA_Mask_3.IA_Mask_3"))
  ;[0.15 0 0.08376 0.5] Input Logic
  (Development|PrintString "Mask 3 Equipped"))

(event Input|EnhancedActionEvents|EnhancedInputActionIA_Mask_4
  (params (ActionValue :type Boolean) (ElapsedSeconds :type Float%20%28double-precision%29) (TriggeredSeconds :type Float%20%28double-precision%29) (InputAction :type Input%20Action%20Object%20Reference :default "/Game/Characters/Player/IA_Mask_4.IA_Mask_4"))
  ;[0.15 0 0.08376 0.5] Input Logic
  (Development|PrintString "Mask 4 Equipped"))

(event Input|EnhancedActionEvents|EnhancedInputActionIA_Pause
  (params (ActionValue :type Boolean) (ElapsedSeconds :type Float%20%28double-precision%29) (TriggeredSeconds :type Float%20%28double-precision%29) (InputAction :type Input%20Action%20Object%20Reference :default "/Game/ThirdPerson/Input/Actions/IA_Pause.IA_Pause"))
  (bind _returnvalue (Game|GetPlayerController 0))
  (bind _returnvalue_2 (Game|GetPlayerController 0))
  ;[0.15 0.15 0.15 0.5] Pause Game
  (:Started
    (Utilities|IsValid (Variables|Default|GetPauseRef)
      (:Is%20Valid
        _)
      (:Is%20Not%20Valid
        (bind _returnvalue_3 (UserInterface|CreateWidget "/Game/UI/PauseMenu/WB_Pause.WB_Pause_C"))
        (Variables|Default|SetPauseRef _returnvalue_3)))
    (if (Game|IsGamePaused)
      (Widget|RemovefromParent (Variables|Default|GetPauseRef))
      (Game|SetGamePaused false)
      (Variables|/Script/Engine.PlayerController|SetbShowMouseCursor _returnvalue false)
      (Input|SetInputModeGameOnly _returnvalue false)
      (else
        (UserInterface|Viewport|AddtoViewport (Variables|Default|GetPauseRef) 0)
        (Game|SetGamePaused true)
        (Variables|/Script/Engine.PlayerController|SetbShowMouseCursor _returnvalue_2 true)
        (Input|SetInputModeGameandUI _returnvalue_2 (Variables|Default|GetPauseRef) "DoNotLock" true false)))))

(event EventBeginPlay
  (Variables|Default|SetTargetControlPoint (CallFunction|GetNearestControlPoint))
  (Development|PrintString "PLAYER SPAWNED")
  ;[0 0.15 0.05668 0.5] Initializing Life to MaxLife
  (Variables|Default|SetCurrentLife (Variables|Default|GetMaximumLife))
  (Development|PrintString "Life Initialized")
  (bind _returnvalue (Game|ConstructObjectfromClass "/Game/UI/PlayerHUD/PelletScore.PelletScore_C"))
  (UserInterface|Viewport|AddtoViewport _returnvalue 0))

(event Collision|EventActorBeginOverlap
  (params (OtherActor :type Actor%20Object%20Reference))
  (Utilities|FlowControl|Sequence
    (:then_0
      ;[0 0.15 0.0306 0.5] Player Overlaps with Enemy
      (bind _asbp_enemy (Utilities|Casting|CastToBP_Enemy OtherActor)
        (:then
          (switch Utilities|FlowControl|Switch|SwitchonEDamageState (Variables|/Game/Blueprints/BP_BaseCharacter.BP_BaseCharacter_C|GetDamageState _asbp_enemy)
            (:NewEnumerator0
              (if (Utilities|Enum|Equal(Enum) (Variables|Default|GetMaskState) (Variables|/Game/Blueprints/BP_BaseCharacter.BP_BaseCharacter_C|GetMaskState _asbp_enemy))
                (Development|PrintString "Masks are the same, Do nothing.")
                (else
                  (Development|PrintString "Masks are different, player loses a life.")
                  ;;[0.15 0.0375 0.01425 0.5] Loss of Life Logic
                  (bind _output_get (Variables|Default|SetCurrentLife (- (Variables|Default|GetCurrentLife) 1)))
                  (if (<= _output_get 0)
                    (Development|PrintString "Player is Dead")
                    (else
                      (Development|PrintString "Player has lost 1 Life"))))))
            (:NewEnumerator1
              (Default|Die _asbp_enemy))))
        (:CastFailed
          ;[0.15 0.1303 0 0.5] Pellet Collection. Standard Pellet +1, Power Pellet +3. Power Pellet should change Enemy State to Vulnerable
          (Class|KismetSystemLibrary|IsObjectOfSoftClass OtherActor "/Game/Blueprints/Pellets/BP_Pellet_Power.BP_Pellet_Power_C"
            (:True
              (Variables|Default|SetPelletsCollected (+ (Variables|Default|GetPelletsCollected) 3))
              (Development|PrintString "Power Pellet Collected")
              (Development|PrintString (Utilities|String|ToString(Integer) (Variables|Default|GetPelletsCollected)))
              (Actor|DestroyActor OtherActor)
              (bind _outactors (Actor|GetAllActorsOfClass "/Game/Blueprints/BP_Enemy.BP_Enemy_C"))
              (for _array_element _outactors
                (Variables|/Game/Blueprints/BP_BaseCharacter.BP_BaseCharacter_C|SetDamageState _array_element "NewEnumerator1"))
              ;;[0 0.1477 0.15 0.5] After Delay, Switch all enemy states back to Default.
              (Utilities|FlowControl|Delay 6.0)
              (bind _outactors_2 (Actor|GetAllActorsOfClass "/Game/Blueprints/BP_BaseCharacter.BP_BaseCharacter_C"))
              (for _array_element_2 _outactors_2
                (Variables|/Game/Blueprints/BP_BaseCharacter.BP_BaseCharacter_C|SetDamageState _array_element_2 "NewEnumerator0")))
            (:False
              (Class|KismetSystemLibrary|IsObjectOfSoftClass OtherActor "/Game/Blueprints/Pellets/BP_Pellet_Base.BP_Pellet_Base_C"
                (:True
                  (Variables|Default|SetPelletsCollected (+ (Variables|Default|GetPelletsCollected) 1))
                  (Development|PrintString (Utilities|String|ToString(Integer) (Variables|Default|GetPelletsCollected)))
                  (Actor|DestroyActor OtherActor))))))))
    (:then_1
      ;[0.15 0.0034 0.1429 0.5] Checks for existing tag on Mask, if it exists, it updates the SMaskInventoryStruct value for that Mask to be TRUE. If true, it should be able to be equipped via Input.
      (Class|KismetSystemLibrary|IsObjectOfSoftClass OtherActor "/Game/Blueprints/Masks/BP_Mask_Base.BP_Mask_Base_C"
        (:True
          (bind _asbp_mask_base (Utilities|Casting|CastToBP_Mask_Base OtherActor))
          (|SwitchGameplayTag (Utilities|Array|Get(acopy) (.gameplaytags (Variables|/Game/Blueprints/Masks/BP_Mask_Base.BP_Mask_Base_C|GetMaskTagContainer _asbp_mask_base)))
            (:Mask.Type.Red
              (Variables|Default|SetMaskInventory (Utilities|Struct|MakeS_MaskInventory true (.blue (Variables|Default|GetMaskInventory)) (.green (Variables|Default|GetMaskInventory)) (.yellow (Variables|Default|GetMaskInventory)))))
            (:Mask.Type.Blue
              (Variables|Default|SetMaskInventory (Utilities|Struct|MakeS_MaskInventory (.red (Variables|Default|GetMaskInventory)) true (.green (Variables|Default|GetMaskInventory)) (.yellow (Variables|Default|GetMaskInventory)))))
            (:Mask.Type.Green
              (Variables|Default|SetMaskInventory (Utilities|Struct|MakeS_MaskInventory (.red (Variables|Default|GetMaskInventory)) (.blue (Variables|Default|GetMaskInventory)) true (.yellow (Variables|Default|GetMaskInventory)))))
            (:Mask.Type.Yellow
              (Variables|Default|SetMaskInventory (Utilities|Struct|MakeS_MaskInventory (.red (Variables|Default|GetMaskInventory)) (.blue (Variables|Default|GetMaskInventory)) (.green (Variables|Default|GetMaskInventory)) true))))
          (Actor|DestroyActor _asbp_mask_base))))))

(event EventTick
  (params (DeltaSeconds :type Float%20%28single-precision%29))
  (CallFunction|MoveTowardControlPoint DeltaSeconds))

(fn ConstructionScript)

(fn OnReachControlPoint
  (bind (_bexists _controlpoint) (Default|GetAdjacent (Variables|Default|GetTargetControlPoint) (Variables|Default|GetDesiredDirection) (Variables|Default|GetMaskState)))
  (if _bexists
    (Variables|Default|SetPreviousControlPoint (Variables|Default|GetTargetControlPoint))
    (Variables|Default|SetTargetControlPoint _controlpoint)
    (Variables|Default|SetCurrentDirection (Variables|Default|GetDesiredDirection))
    (else
      (bind (_bexists_2 _controlpoint_2) (Default|GetAdjacent (Variables|Default|GetTargetControlPoint) (Variables|Default|GetCurrentDirection) (Variables|Default|GetMaskState)))
      (if _bexists_2
        (Variables|Default|SetPreviousControlPoint (Variables|Default|GetTargetControlPoint))
        (Variables|Default|SetTargetControlPoint _controlpoint_2)
        (else
          (Variables|Default|SetCurrentDirection "NewEnumerator4"))))))