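; Test player Blueprint that prototypes movement, mask matching and pausing, with debug prints standing in for most gameplay outcomes.
; Enhanced Input moves the actor by per-trigger world offsets, while the four mask inputs only print without changing MaskState.
; Overlaps compare MaskState against enemies or detect pellets, printing the result.
; The pause input creates and reuses a WB_Pause widget, toggling game pause, cursor and input mode.
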(event Input|EnhancedActionEvents|EnhancedInputActionIA_Move_Up
  (params (ActionValue :type Float%20%28double-precision%29) (ElapsedSeconds :type Float%20%28double-precision%29) (TriggeredSeconds :type Float%20%28double-precision%29) (InputAction :type Input%20Action%20Object%20Reference :default "/Game/Characters/Player/IA_Move_Up.IA_Move_Up"))
  ;[0.15 0 0.08376 0.5] Input Logic
  (:Triggered
    (Transformation|AddActorWorldOffset (Math|Vector|MakeVector (* ActionValue 1.0) 0.0 0.0)))
  (:Completed
    (Development|PrintString "IA_Move_Up Released.")))

(event Input|EnhancedActionEvents|EnhancedInputActionIA_Move_Right
  (params (ActionValue :type Float%20%28double-precision%29) (ElapsedSeconds :type Float%20%28double-precision%29) (TriggeredSeconds :type Float%20%28double-precision%29) (InputAction :type Input%20Action%20Object%20Reference :default "/Game/Characters/Player/IA_Move_Right.IA_Move_Right"))
  ;[0.15 0 0.08376 0.5] Input Logic
  (:Triggered
    (Transformation|AddActorWorldOffset (Math|Vector|MakeVector 0.0 (* ActionValue 1.0) 0.0)))
  (:Completed
    (Development|PrintString "IA_Move_Right Released.")))

(event Input|EnhancedActionEvents|EnhancedInputActionIA_Mask_1
  (params (ActionValue :type Boolean) (ElapsedSeconds :type Float%20%28double-precision%29) (TriggeredSeconds :type Float%20%28double-precision%29) (InputAction :type Input%20Action%20Object%20Reference :default "/Game/Characters/Player/IA_Mask_1.IA_Mask_1"))
  ;[0.15 0 0.08376 0.5] Input Logic
  (Development|PrintString "Mask 1 Equipped"))

(event Input|EnhancedActionEvents|EnhancedInputActionIA_Mask_2
  (params (ActionValue :type Boolean) (ElapsedSeconds :type Float%20%28double-precision%29) (TriggeredSeconds :type Float%20%28double-precision%29) (InputAction :type Input%20Action%20Object%20Reference :default "/Game/Characters/Player/IA_Mask_2.IA_Mask_2"))
  ;[0.15 0 0.08376 0.5] Input Logic
  (Development|PrintString "Mask 2 Equipped"))

(event Input|EnhancedActionEvents|EnhancedInputActionIA_Mask_3
  (params (ActionValue :type Boolean) (ElapsedSeconds :type Float%20%28double-precision%29) (TriggeredSeconds :type Float%20%28double-precision%29) (InputAction :type Input%20Action%20Object%20Reference :default "/Game/Characters/Player/IA_Mask_3.IA_Mask_3"))
  ;[0.15 0 0.08376 0.5] Input Logic
  (Development|PrintString "Mask 3 Equipped"))

(event Input|EnhancedActionEvents|EnhancedInputActionIA_Mask_4
  (params (ActionValue :type Boolean) (ElapsedSeconds :type Float%20%28double-precision%29) (TriggeredSeconds :type Float%20%28double-precision%29) (InputAction :type Input%20Action%20Object%20Reference :default "/Game/Characters/Player/IA_Mask_4.IA_Mask_4"))
  ;[0.15 0 0.08376 0.5] Input Logic
  (Development|PrintString "Mask 4 Equipped"))

(event Input|EnhancedActionEvents|EnhancedInputActionIA_Pause
  (params (ActionValue :type Boolean) (ElapsedSeconds :type Float%20%28double-precision%29) (TriggeredSeconds :type Float%20%28double-precision%29) (InputAction :type Input%20Action%20Object%20Reference :default "/Game/ThirdPerson/Input/Actions/IA_Pause.IA_Pause"))
  (bind _returnvalue (Game|GetPlayerController 0))
  (bind _returnvalue_2 (Game|GetPlayerController 0))
  ;[0.15 0.15 0.15 0.5] Pause Game
  (:Started
    (Utilities|IsValid (Variables|Default|GetPauseRef)
      (:Is%20Valid
        _)
      (:Is%20Not%20Valid
        (bind _returnvalue_3 (UserInterface|CreateWidget "/Game/UI/PauseMenu/WB_Pause.WB_Pause_C"))
        (Variables|Default|SetPauseRef _returnvalue_3)))
    (if (Game|IsGamePaused)
      (Widget|RemovefromParent (Variables|Default|GetPauseRef))
      (Game|SetGamePaused false)
      (Variables|/Script/Engine.PlayerController|SetbShowMouseCursor _returnvalue false)
      (Input|SetInputModeGameOnly _returnvalue false)
      (else
        (UserInterface|Viewport|AddtoViewport (Variables|Default|GetPauseRef) 0)
        (Game|SetGamePaused true)
        (Variables|/Script/Engine.PlayerController|SetbShowMouseCursor _returnvalue_2 true)
        (Input|SetInputModeGameandUI _returnvalue_2 (Variables|Default|GetPauseRef) "DoNotLock" true false)))))

(event EventBeginPlay)

(event Collision|EventActorBeginOverlap
  (params (OtherActor :type Actor%20Object%20Reference))
  ;[0 0.15 0.0306 0.5] Player Overlaps with Enemy
  (bind _asbp_enemy_character (Utilities|Casting|CastToBP_Enemy_Character OtherActor)
    (:then
      (if (Utilities|Enum|Equal(Enum) (Variables|Default|GetMaskState) (Variables|/Game/Blueprints/BP_Enemy_Character.BP_Enemy_Character_C|GetMaskState _asbp_enemy_character))
        (Development|PrintString "Masks are the same, Do nothing.")
        (else
          (Development|PrintString "Masks are different, player loses a life."))))
    (:CastFailed
      (Utilities|Casting|CastToBP_Pellet_Base OtherActor)
      (Development|PrintString "Overlapped with a Pellet."))))

(event EventTick
  (params (DeltaSeconds :type Float%20%28single-precision%29)))

(fn ConstructionScript)