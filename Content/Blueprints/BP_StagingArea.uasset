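; BP_StagingArea is an area actor that spawns BP_Enemy instances at random spots within its bounds and assigns each a mask state.
; Random spots are offset from the Center component using the actor's bounds extent inset by a margin, with height lowered by that inset extent.
; It exposes getters for its center and linked entrance control point.
; A debug event spawns one enemy with a fixed mask state.
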(event Custom|DebugSpawnEnemy
  (CallFunction|SpawnEnemy "NewEnumerator1"))

(event EventBeginPlay)

(event Collision|EventActorBeginOverlap
  (params (OtherActor :type Actor%20Object%20Reference)))

(event EventTick
  (params (DeltaSeconds :type Float%20%28single-precision%29)))

(fn ConstructionScript)

(fn GetCenterLocation
  (return (Transformation|GetWorldLocation (Variables|Default|GetCenter))))

(fn GetEntranceLocation
  (Utilities|IsValid (Variables|Default|GetEntranceControlPoint)
    (:Is%20Valid
      (return (Transformation|GetActorLocation (Variables|Default|GetEntranceControlPoint))))))

(fn SpawnEnemy
  (params (MaskState :type EMaskState%20Enum :default "NewEnumerator0"))
  (bind _returnvalue (Game|SpawnActorfromClass "/Game/Blueprints/BP_Enemy.BP_Enemy_C" (Math|Transform|MakeTransform (CallFunction|GetRandomStageSpot) "0, 0, 0" "1.000000,1.000000,1.000000") "Undefined" "MultiplyWithRoot" 0 0))
  (Variables|/Game/Blueprints/BP_BaseCharacter.BP_BaseCharacter_C|SetMaskState _returnvalue MaskState))

(fn GetRandomStageSpot
  (bind _boxextent (Collision|GetActorBounds false false))
  (bind _returnvalue (- _boxextent 1e+02))
  (bind _returnvalue_2 (* _returnvalue 2.0))
  (bind (_x _y) (Math|Vector|BreakVector _returnvalue_2))
  (return (- (+ (CallFunction|GetCenterLocation) (Math|Vector|MakeVector (* (Math|Random|RandomFloat) _x) (* (Math|Random|RandomFloat) _y) 0.0)) _returnvalue)))