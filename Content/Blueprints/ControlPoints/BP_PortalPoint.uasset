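; BP_PortalPoint is a control point that moves characters to its ConnectedPortal.
; TransferThroughPortal teleports a character there, retargets it along the destination's first Adjacent direction, and syncs a player's DesiredDirection.
; The destination briefly blacklists the arriving character to prevent an immediate bounce back.
; The Box overlap event is empty and its transfer logic is disconnected, so this file never triggers the transfer itself.
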(event OnComponentBeginOverlap(Box)
  (params (OverlappedComponent :type Primitive%20Component%20Object%20Reference) (OtherActor :type Actor%20Object%20Reference) (OtherComp :type Primitive%20Component%20Object%20Reference) (OtherBodyIndex :type Integer) (bFromSweep :type Boolean) (SweepResult :type Hit%20Result%20Structure%20%28by%20ref%29)))

(event Custom|BlacklistCharacter
  (params (TargetCharacter :type BP%20Base%20Character%20Object%20Reference))
  (Utilities|Set|Add (Variables|Default|GetBlacklist) TargetCharacter)
  (Utilities|FlowControl|Delay 0.1)
  (Utilities|Set|Remove (Variables|Default|GetBlacklist) TargetCharacter))

(fn ConstructionScript
  (|CallParentFunction))

(fn TransferThroughPortal
  (params (TargetCharacter :type BP%20Base%20Character%20Object%20Reference))
  (bind _connectedportal (Variables|Default|GetConnectedPortal))
  (bind _adjacent (Variables|/Game/Blueprints/ControlPoints/BP_ControlPoint.BP_ControlPoint_C|GetAdjacent _connectedportal))
  (if (not (Utilities|Set|Contains (Variables|Default|GetBlacklist) TargetCharacter))
    (CallFunction|BlacklistCharacter (Variables|Default|GetConnectedPortal) TargetCharacter)
    (bind _keys (Utilities|Map|Keys _adjacent))
    (Variables|/Game/Blueprints/BP_BaseCharacter.BP_BaseCharacter_C|SetCurrentDirection TargetCharacter (Utilities|Array|Get(acopy) _keys))
    (Variables|/Game/Blueprints/BP_BaseCharacter.BP_BaseCharacter_C|SetTargetControlPoint TargetCharacter (.Value (Utilities|Map|Find _adjacent (Utilities|Array|Get(acopy) _keys))))
    (Variables|/Game/Blueprints/BP_BaseCharacter.BP_BaseCharacter_C|SetPreviousControlPoint TargetCharacter (Variables|Default|GetConnectedPortal))
    (Transformation|SetActorLocation TargetCharacter (Transformation|GetActorLocation (Variables|Default|GetConnectedPortal)) false false)
    (bind _asbp_player (Utilities|Casting|CastToBP_Player TargetCharacter))
    (Variables|/Game/Characters/Player/BP_Player.BP_Player_C|SetDesiredDirection _asbp_player (Variables|/Game/Blueprints/BP_BaseCharacter.BP_BaseCharacter_C|GetCurrentDirection TargetCharacter))))