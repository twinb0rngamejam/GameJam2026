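; BP_Pellet_Power is a power pellet that makes enemies vulnerable when consumed.
; It overrides OnConsumed, calls the parent behavior, then gathers every BP_Enemy in the level with GetAllActorsOfClass and calls BecomeVulnerable on each.
; BeginPlay, overlap and Tick nodes are disabled, and the construction script only calls its parent.
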(event EventBeginPlay
  (|CallParentFunction) ; This node is disabled and will not be called.\nDrag off pins to build functionality.
)

(event Collision|EventActorBeginOverlap
  (params (OtherActor :type Actor%20Object%20Reference))
  (|CallParentFunction OtherActor) ; This node is disabled and will not be called.\nDrag off pins to build functionality.
)

(event EventTick
  (params (DeltaSeconds :type Float%20%28single-precision%29))
  (|CallParentFunction DeltaSeconds) ; This node is disabled and will not be called.\nDrag off pins to build functionality.
)

(event EventOnConsumed
  (params (Consumer :type BP%20Player%20Object%20Reference))
  (|CallParentFunction Consumer)
  (bind _outactors (Actor|GetAllActorsOfClass "/Game/Blueprints/BP_Enemy.BP_Enemy_C"))
  (for _array_element _outactors
    (Default|BecomeVulnerable _array_element)))

(fn ConstructionScript
  (|CallParentFunction))