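; Pellet-priced lock that opens a blocked direction on a linked control point when the player touches it.
; On box overlap it checks the player's collected pellets against the price and that a control point is assigned, printing an error if none is.
; Purchase deducts the pellets, calls UnlockDirection on the control point, destroys the listed actors, then destroys the lock itself.
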(event OnComponentBeginOverlap(Box)
  (params (OverlappedComponent :type Primitive%20Component%20Object%20Reference) (OtherActor :type Actor%20Object%20Reference) (OtherComp :type Primitive%20Component%20Object%20Reference) (OtherBodyIndex :type Integer) (bFromSweep :type Boolean) (SweepResult :type Hit%20Result%20Structure%20%28by%20ref%29))
  (Utilities|Casting|CastToBP_Player OtherActor)
  (if (CallFunction|HasEnoughPellets)
    (Utilities|IsValid (Variables|Lock|GetControlPoint)
      (:Is%20Valid
        (CallFunction|Purchase))
      (:Is%20Not%20Valid
        (Development|PrintString (Utilities|String|Append "ERROR: No control point attached to purchasable lock " (Utilities|GetDisplayName self)) true false "(R=1.000000,G=0.053122,B=0.000000,A=1.000000)")))))

(event Custom|Purchase
  ;[0.15 0.15 0.15 0.5] Purchase Logic - Remove pellets from player, unlock control point direction, destroy misc actors
  (Variables|/Game/Characters/Player/BP_Player.BP_Player_C|SetPelletsCollected (Variables|Default|GetPlayer) (- (Variables|/Game/Characters/Player/BP_Player.BP_Player_C|GetPelletsCollected (Variables|Default|GetPlayer)) (Variables|Lock|GetPrice)))
  (Default|UnlockDirection (Variables|Lock|GetControlPoint) (Variables|Lock|GetLockDirection))
  (for _array_element (Variables|Lock|GetDestroyedActorsWhenUnlocked)
    (Actor|DestroyActor _array_element))
  (Development|PrintString "Purchasable Unlocked! " true false)
  (Actor|DestroyActor))

(event EventBeginPlay
  (bind _returnvalue (Actor|GetActorOfClass "/Game/Characters/Player/BP_Player.BP_Player_C"))
  (Variables|Default|SetPlayer _returnvalue))

(fn ConstructionScript)

(fn HasEnoughPellets
  (return (>= (Variables|/Game/Characters/Player/BP_Player.BP_Player_C|GetPelletsCollected (Variables|Default|GetPlayer)) (Variables|Lock|GetPrice))))