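; BP_LevelExitLock is a level actor that unlocks the exit once every mask in the level has been picked up.
; On BeginPlay it counts all BP_Mask_Base actors and binds to the player's OnMaskPickup event, decrementing the count on each pickup.
; At zero it unlocks the configured direction on its ControlPoint and destroys the listed blocker actors, or prints an error if no control point is valid.
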(event Custom|OnMaskPickup
  (params (MaskState :type EMaskState%20Enum :default "NewEnumerator0"))
  (bind _result (Math|Integer|DecrementInt (Variables|Default|GetNumMasks))
    (:%20%20
      (if (<= _result 0)
        (Utilities|IsValid (Variables|MaskLock|GetControlPoint)
          (:Is%20Valid
            (Default|UnlockDirection (Variables|MaskLock|GetControlPoint) (Variables|MaskLock|GetUnlockedDirection))
            (Development|PrintString "Exit Unlocked!" true false "(R=0.000000,G=0.660000,B=1.000000,A=1.000000)" 5.0)
            (for _array_element (Variables|Default|GetActorsDestroyedOnUnlock)
              (Actor|DestroyActor _array_element)))
          (:Is%20Not%20Valid
            (Development|PrintString "ERROR: No control point lock attached to level exit lock actor" true false "(R=1.000000,G=0.014456,B=0.000000,A=1.000000)" 5.0)))))))

(event EventBeginPlay
  (bind _outactors (Actor|GetAllActorsOfClass "/Game/Blueprints/Masks/BP_Mask_Base.BP_Mask_Base_C"))
  (Variables|Default|SetNumMasks (Utilities|Array|Length _outactors))
  (bind _returnvalue (Actor|GetActorOfClass "/Game/Characters/Player/BP_Player.BP_Player_C"))
  (EventDispatchers|BindEventtoOnMaskPickup _returnvalue (delegate Custom|OnMaskPickup)))

(fn ConstructionScript)