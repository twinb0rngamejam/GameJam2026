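; Enemy that navigates a network of control points toward or away from the player, with a staging area where it rests at start and after dying.
; On reaching a point, its behavior picks the next direction: random walk, chase, flee or return to stage.
; Timers alternate wandering and chasing, while vulnerability triggers fleeing.
; A ScriptedMove macro loops each tick to handle staging-area entry and exit.
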(event Custom|BecomeVulnerable
  (bind _targetplayer (Variables|Default|GetTargetPlayer))
  (bind _returnvalue (Transformation|GetActorLocation _targetplayer))
  (switch Utilities|FlowControl|Switch|SwitchonEDamageState (Variables|Default|GetDamageState)
    (:NewEnumerator0
      _)
    (:NewEnumerator1
      _))
  (CallFunction|SetDamageState "NewEnumerator1")
  (Utilities|FlowControl|Sequence
    (:then_0
      (switch Utilities|FlowControl|Switch|SwitchonEEnemyBehavior (Variables|Default|GetCurrentBehavior)
        (:NewEnumerator0
          _)
        (:NewEnumerator1
          _)
        (:NewEnumerator2
          _))
      (CallFunction|SetBehavior "NewEnumerator2")
      (if (< (Math|Vector|Distance(Vector) (+ (Transformation|GetActorLocation) (CallFunction|DirectiontoVector (Variables|Default|GetCurrentDirection))) _returnvalue) (Math|Vector|Distance(Vector) _returnvalue (Transformation|GetActorLocation)))
        (CallFunction|ImmediateTurn)))
    (:then_1
      (Utilities|FlowControl|Delay (Variables|Default|GetVulnerabilityDuration))
      (CallFunction|StopVulnerability))))

(event Custom|StopVulnerability
  (switch Utilities|FlowControl|Switch|SwitchonEDamageState (Variables|Default|GetDamageState)
    (:NewEnumerator0
      _)
    (:NewEnumerator1
      _))
  (CallFunction|SetDamageState "NewEnumerator0")
  (switch Utilities|FlowControl|Switch|SwitchonEEnemyBehavior (Variables|Default|GetCurrentBehavior)
    (:NewEnumerator2
      (CallFunction|SetBehavior "NewEnumerator0"))))

(event Custom|EnterStagingArea
  ;[0.15 0.000336 0.1258 0.5] Enter Staging Area
  (CallFunction|SetBehavior "NewEnumerator5")
  (Utilities|ScriptedMove (CallFunction|GetStagingAreaEntranceLocation self) (Variables|Default|GetStagingSpeed)
    (:LocationReached
      (Utilities|ScriptedMove (CallFunction|GetStagingAreaCenterLocation self) (Variables|Default|GetStagingSpeed)
        (:LocationReached
          (Utilities|ScriptedMove (+ (CallFunction|GetStagingAreaCenterLocation self) (Variables|Default|GetStagingRestOffset)) (Variables|Default|GetStagingSpeed)
            (:LocationReached
              (CallFunction|SetDamageState "NewEnumerator0")
              (Utilities|FlowControl|Delay (Variables|Default|GetStageRestTime))
              (CallFunction|ExitStagingArea))))))))

(event Custom|OnBehaviorChanged
  (params (NewBehavior :type EEnemyBehavior%20Enum :default "NewEnumerator0") (PreviousBehavior :type EEnemyBehavior%20Enum :default "NewEnumerator0"))
  (switch Utilities|FlowControl|Switch|SwitchonEEnemyBehavior NewBehavior
    (:NewEnumerator0
      (Utilities|FlowControl|Delay 5.0)
      (CallFunction|StartChase))
    (:NewEnumerator1
      (Utilities|FlowControl|Delay 5.0)
      (CallFunction|StopChase))))

(event Custom|ExitStagingArea
  ;[0.15 0.01268 0 0.5] Exit Staging Area
  (Utilities|ScriptedMove (CallFunction|GetStagingAreaCenterLocation self) (Variables|Default|GetStagingSpeed)
    (:LocationReached
      (Utilities|ScriptedMove (CallFunction|GetStagingAreaEntranceLocation self) (Variables|Default|GetStagingSpeed)
        (:LocationReached
          (Variables|Default|SetTargetControlPoint (CallFunction|GetStagingAreaControlPoint self))
          (Variables|Default|SetPreviousControlPoint 0)
          (CallFunction|SetBehavior "NewEnumerator0"))))))

(event Custom|StartChase
  (switch Utilities|FlowControl|Switch|SwitchonEEnemyBehavior (Variables|Default|GetCurrentBehavior)
    (:NewEnumerator0
      (CallFunction|SetBehavior "NewEnumerator1"))))

(event Custom|StopChase
  (switch Utilities|FlowControl|Switch|SwitchonEEnemyBehavior (Variables|Default|GetCurrentBehavior)
    (:NewEnumerator1
      (CallFunction|SetBehavior "NewEnumerator0"))))

(event Custom|Die
  (CallFunction|SetDamageState "NewEnumerator2")
  (CallFunction|SetBehavior "NewEnumerator4"))

(event EventBeginPlay
  (bind _returnvalue (Actor|GetActorOfClass "/Game/Characters/Player/BP_Player.BP_Player_C"))
  (bind _output_get (Variables|Default|SetTargetPlayer _returnvalue))
  (Utilities|IsValid _output_get
    (:Is%20Valid
      _)
    (:Is%20Not%20Valid
      (Development|PrintString "ERROR: Enemy could not find player" true false "(R=1.000000,G=0.018078,B=0.000000,A=1.000000)")))
  (Utilities|IsValid (Variables|Default|GetTargetControlPoint)
    (:Is%20Valid
      _)
    (:Is%20Not%20Valid
      (Variables|Default|SetTargetControlPoint (CallFunction|GetNearestControlPoint))))
  ;[0.15 0.15 0.15 0.5] Assumes enemy starts in staging area (Which it should)
  (Variables|Default|SetStagingRestOffset (- (Transformation|GetActorLocation) (CallFunction|GetStagingAreaCenterLocation self)))
  (Utilities|FlowControl|Delay (Variables|Default|GetStageRestTime))
  (CallFunction|ExitStagingArea))

(fn ConstructionScript
  (|CallParentFunction))

(fn OnReachControlPoint
  (switch Utilities|FlowControl|Switch|SwitchonEEnemyBehavior (Variables|Default|GetCurrentBehavior)
    (:NewEnumerator0
      ;[0.15 0.15 0.15 0.5] When reaching a control point, get its available directions, pick one of those, get the associated control point, switch direction and target
      (Utilities|IsValid (Variables|Default|GetTargetControlPoint) :!label _label
        (:Is%20Valid
          (bind _returnvalue (Default|GetAvailableDirections (Variables|Default|GetTargetControlPoint)))
          (LocalVariables|SetNewDirection (CallFunction|SelectNextDirection _returnvalue))
          (bind (_bexists _controlpoint) (Default|GetAdjacent (Variables|Default|GetTargetControlPoint) (LocalVariables|GetNewDirection)))
          (if _bexists
            (Variables|Default|SetCurrentDirection (LocalVariables|GetNewDirection))
            (Variables|Default|SetPreviousControlPoint (Variables|Default|GetTargetControlPoint))
            (Variables|Default|SetTargetControlPoint _controlpoint)
            (else
              (Development|PrintString (Utilities|String|Append "ERROR: Control Point " (Utilities|GetDisplayName (Variables|Default|GetTargetControlPoint)) " has no Control Point associated with key " (Utilities|String|EnumtoString (LocalVariables|GetNewDirection))) true true "(R=1.000000,G=0.000100,B=0.025815,A=1.000000)" 5.0) ; Should never happen unless a key was added and not filled with a control point
            )))))
    (:NewEnumerator1
      (goto _label))
    (:NewEnumerator2
      (goto _label))
    (:NewEnumerator4
      (if (!= (Variables|Default|GetTargetControlPoint) (CallFunction|GetStagingAreaControlPoint self))
        (goto _label)
        (else
          ;[0.15 0.15 0.15 0.5] Rest
          (CallFunction|EnterStagingArea))))))

(fn SelectNextDirection
  (params (AvailableDirections :type Array%20of%20EMoveDirection%20Enums :default "NewEnumerator0"))
  (switch Utilities|FlowControl|Switch|SwitchonEEnemyBehavior (Variables|Default|GetCurrentBehavior)
    (:NewEnumerator0
      ;[0.15 0.15 0.15 0.5] Random walk: Take a random available direction that isn't turning around, unless that's the only choice
      (bind _output_get (LocalVariables|SetDirections AvailableDirections))
      (Utilities|Array|RemoveItem _output_get (CallFunction|GetOppositeDirection (Variables|Default|GetCurrentDirection)))
      (if (> (.OutIndex (Utilities|Array|Random (LocalVariables|GetDirections))) -1)
        (return (.OutItem (Utilities|Array|Random (LocalVariables|GetDirections))))
        (else
          (return (CallFunction|GetOppositeDirection (Variables|Default|GetCurrentDirection))))))
    (:NewEnumerator1
      ;[0.15 0.15 0.15 0.5] Chase: Take the direction that brings the enemy closest to the player
      (return (CallFunction|GetDirectiontoControlPoint (CallFunction|GetControlPointClosesttoLocation (Transformation|GetActorLocation (Variables|Default|GetTargetPlayer))))))
    (:NewEnumerator2
      ;[0.15 0.15 0.15 0.5] Flee: Take the direction that brings the enemy furthest from the player
      (return (CallFunction|GetDirectiontoControlPoint (CallFunction|GetFurthestControlPointfromLocation (Transformation|GetActorLocation (Variables|Default|GetTargetPlayer))))))
    (:NewEnumerator4
      ;[0.15 0.15 0.15 0.5] Return to Stage: Take the direction that brings enemy to the Staging Area Entrance
      (return (CallFunction|GetDirectiontoControlPoint (CallFunction|GetStagingAreaControlPoint self))))))