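; Base enemy character, a Pac-Man-style ghost that moves between linked BP_ControlPoint actors in random walk, chase, flee or return-to-stage behavior.
; Tick moves it toward its target point, where it picks the next direction randomly or by a greedy distance heuristic.
; Damage states swap the mask material: vulnerability triggers a timed flee, and death sends it back to the staging area.
; A latent ScriptedMove macro loops each tick to drive staging entry, rest and exit.
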(event Custom|BecomeVulnerable
  (bind _targetplayer (Variables|Movement|GetTargetPlayer))
  (bind _returnvalue (Transformation|GetActorLocation _targetplayer))
  ;[0.15 0.15 0.15 0.5] Start Vulnerability
  (switch Utilities|FlowControl|Switch|SwitchonEDamageState (Variables|Default|GetDamageState)
    (:NewEnumerator0
      _)
    (:NewEnumerator1
      _))
  (StateManagement|SetDamageState "NewEnumerator1")
  (Utilities|FlowControl|Sequence
    (:then_0
      (switch Utilities|FlowControl|Switch|SwitchonEEnemyBehavior (Variables|Movement|GetCurrentBehavior)
        (:NewEnumerator0
          _)
        (:NewEnumerator1
          _)
        (:NewEnumerator2
          _))
      (StateManagement|SetBehavior "NewEnumerator2")
      (if (< (Math|Vector|Distance(Vector) (+ (Transformation|GetActorLocation) (CallFunction|DirectiontoVector (Variables|Movement|GetCurrentDirection))) _returnvalue) (Math|Vector|Distance(Vector) _returnvalue (Transformation|GetActorLocation)))
        (CallFunction|ImmediateTurn)))
    (:then_1
      (Utilities|FlowControl|Delay (Variables|Default|GetVulnerabilityDuration))
      (CallFunction|StopVulnerability))))

(event Custom|StopVulnerability
  ;[0.15 0.15 0.15 0.5] Stop Vulnerability
  (switch Utilities|FlowControl|Switch|SwitchonEDamageState (Variables|Default|GetDamageState)
    (:NewEnumerator0
      _)
    (:NewEnumerator1
      _))
  (StateManagement|SetDamageState "NewEnumerator0")
  (switch Utilities|FlowControl|Switch|SwitchonEEnemyBehavior (Variables|Movement|GetCurrentBehavior)
    (:NewEnumerator2
      (StateManagement|SetBehavior "NewEnumerator0"))))

(event Custom|EnterStagingArea
  ;[0.15 0.000336 0.1258 0.5] Enter Staging Area
  (StateManagement|SetBehavior "NewEnumerator5")
  (Utilities|ScriptedMove (CallFunction|GetStagingAreaEntranceLocation self) (Variables|Staging|GetStagingSpeed)
    (:LocationReached
      (Utilities|ScriptedMove (CallFunction|GetStagingAreaCenterLocation self) (Variables|Staging|GetStagingSpeed)
        (:LocationReached
          (Utilities|ScriptedMove (+ (CallFunction|GetStagingAreaCenterLocation self) (Variables|Staging|GetStagingRestOffset)) (Variables|Staging|GetStagingSpeed)
            (:LocationReached
              (StateManagement|SetDamageState "NewEnumerator0")
              (Utilities|FlowControl|Delay (Variables|Staging|GetStageRestTime))
              (CallFunction|ExitStagingArea))))))))

(event Custom|OnBehaviorChanged
  (params (NewBehavior :type EEnemyBehavior%20Enum :default "NewEnumerator0") (PreviousBehavior :type EEnemyBehavior%20Enum :default "NewEnumerator0"))
  (switch Utilities|FlowControl|Switch|SwitchonEEnemyBehavior NewBehavior
    (:NewEnumerator0
      (Utilities|FlowControl|Delay 5.0)
      (CallFunction|StartChase))
    (:NewEnumerator1
      (Utilities|FlowControl|Delay 5.0)
      (CallFunction|StopChase))))

(event Custom|ExitStagingArea
  ;[0.15 0.01268 0 0.5] Exit Staging Area
  (Utilities|ScriptedMove (CallFunction|GetStagingAreaCenterLocation self) (Variables|Staging|GetStagingSpeed)
    (:LocationReached
      (Utilities|ScriptedMove (CallFunction|GetStagingAreaEntranceLocation self) (Variables|Staging|GetStagingSpeed)
        (:LocationReached
          (Variables|Movement|SetTargetControlPoint (CallFunction|GetStagingAreaControlPoint self))
          (Variables|Movement|SetPreviousControlPoint 0)
          (StateManagement|SetBehavior "NewEnumerator0"))))))

(event Custom|TurnAround
  (CallFunction|ImmediateTurn))

(event Custom|StartChase
  (switch Utilities|FlowControl|Switch|SwitchonEEnemyBehavior (Variables|Movement|GetCurrentBehavior)
    (:NewEnumerator0
      (StateManagement|SetBehavior "NewEnumerator1"))))

(event Custom|StopChase
  (switch Utilities|FlowControl|Switch|SwitchonEEnemyBehavior (Variables|Movement|GetCurrentBehavior)
    (:NewEnumerator1
      (StateManagement|SetBehavior "NewEnumerator0"))))

(event Custom|Die
  (StateManagement|SetDamageState "NewEnumerator2")
  (StateManagement|SetBehavior "NewEnumerator4"))

(event EventBeginPlay
  ;[0.15 0.15 0.15 0.5] Begin Play - Set Original Material
  (Variables|Default|SetOriginalMaterial (Rendering|Material|GetMaterial (Variables|Default|GetMaskMesh) 0)))

(event Collision|EventActorBeginOverlap
  (params (OtherActor :type Actor%20Object%20Reference))
  ;[0.15 0.15 0.15 0.5] Overlap: Will determine whether the player should actually be hit later (Also should probably have player detect enemies instead)
  (Utilities|Casting|CastToBP_Player OtherActor)
  (Development|PrintString (Utilities|String|Append (Utilities|GetDisplayName self) " has hit Player") true false))

(event EventTick
  (params (DeltaSeconds :type Float%20%28single-precision%29))
  (StateManagement|UpdateState DeltaSeconds))

(fn ConstructionScript)

(fn MoveTowardControlPoint
  (params (DeltaSeconds :type Float%20%28double-precision%29))
  (Utilities|IsValid (Variables|Movement|GetTargetControlPoint)
    (:Is%20Valid
      (bind _barrived (CallFunction|MoveTowardLocation DeltaSeconds (Variables|Movement|GetMoveSpeed) (Transformation|GetActorLocation (Variables|Movement|GetTargetControlPoint))))
      (if _barrived
        (CallFunction|OnReachControlPoint)))))

(fn OnReachControlPoint
  (switch Utilities|FlowControl|Switch|SwitchonEEnemyBehavior (Variables|Movement|GetCurrentBehavior)
    (:NewEnumerator0
      ;[0.15 0.15 0.15 0.5] When reaching a control point, get its available directions, pick one of those, get the associated control point, switch direction and target
      (Utilities|IsValid (Variables|Movement|GetTargetControlPoint) :!label _label
        (:Is%20Valid
          (bind _returnvalue (Default|GetAvailableDirections (Variables|Movement|GetTargetControlPoint) "NewEnumerator0"))
          (LocalVariables|SetNewDirection (CallFunction|SelectNextDirection _returnvalue))
          (bind (_bexists _controlpoint) (Default|GetAdjacent (Variables|Movement|GetTargetControlPoint) (LocalVariables|GetNewDirection) "NewEnumerator0"))
          (if _bexists
            (Variables|Movement|SetCurrentDirection (LocalVariables|GetNewDirection))
            (Variables|Movement|SetPreviousControlPoint (Variables|Movement|GetTargetControlPoint))
            (Variables|Movement|SetTargetControlPoint _controlpoint)
            (else
              (Development|PrintString (Utilities|String|Append "ERROR: Control Point " (Utilities|GetDisplayName (Variables|Movement|GetTargetControlPoint)) " has no Control Point associated with key " (Utilities|String|EnumtoString (LocalVariables|GetNewDirection))) true true "(R=1.000000,G=0.000100,B=0.025815,A=1.000000)" 5.0) ; Should never happen unless a key was added and not filled with a control point
            )))))
    (:NewEnumerator1
      (goto _label))
    (:NewEnumerator2
      (goto _label))
    (:NewEnumerator4
      (if (!= (Variables|Movement|GetTargetControlPoint) (CallFunction|GetStagingAreaControlPoint self))
        (goto _label)
        (else
          ;[0.15 0.15 0.15 0.5] Rest
          (CallFunction|EnterStagingArea))))))

(fn MoveTowardLocation
  (params (DeltaSeconds :type Float%20%28double-precision%29) (Speed :type Float%20%28double-precision%29) (TargetLocation :type Vector))
  ;[0.15 0.15 0.15 0.5] Will be used for doing specific movements in the staging area (Have it enter the staging area and to its resting location, move to the middle of the staging area then exit)
  (bind _output_get (LocalVariables|SetMoveAmount (* DeltaSeconds Speed)))
  (if (< _output_get (Math|Vector|Distance2D(Vector) TargetLocation (Transformation|GetActorLocation)))
    (Transformation|SetActorLocation (+ (Transformation|GetActorLocation) (* (Math|Vector|GetUnitDirection(Vector) (Transformation|GetActorLocation) TargetLocation) (LocalVariables|GetMoveAmount))) false false)
    (return false)
    (else
      (Transformation|SetActorLocation TargetLocation false false)
      (return true))))

(fn SelectNextDirection
  (params (AvailableDirections :type Array%20of%20EMoveDirection%20Enums :default "NewEnumerator0"))
  (switch Utilities|FlowControl|Switch|SwitchonEEnemyBehavior (Variables|Movement|GetCurrentBehavior)
    (:NewEnumerator0
      ;[0.15 0.15 0.15 0.5] Random walk: Take a random available direction that isn't turning around, unless that's the only choice
      (bind _output_get (LocalVariables|SetDirections AvailableDirections))
      (Utilities|Array|RemoveItem _output_get (CallFunction|GetOppositeDirection (Variables|Movement|GetCurrentDirection)))
      (if (> (.OutIndex (Utilities|Array|Random (LocalVariables|GetDirections))) -1)
        (return (.OutItem (Utilities|Array|Random (LocalVariables|GetDirections))))
        (else
          (return (CallFunction|GetOppositeDirection (Variables|Movement|GetCurrentDirection))))))
    (:NewEnumerator1
      ;[0.15 0.15 0.15 0.5] Chase: Take the direction that brings the enemy closest to the player
      (return (CallFunction|GetDirectiontoControlPoint (CallFunction|GetControlPointClosesttoLocation (Transformation|GetActorLocation (Variables|Movement|GetTargetPlayer))))))
    (:NewEnumerator2
      ;[0.15 0.15 0.15 0.5] Flee: Take the direction that brings the enemy furthest from the player
      (return (CallFunction|GetDirectiontoControlPoint (CallFunction|GetFurthestControlPointfromLocation (Transformation|GetActorLocation (Variables|Movement|GetTargetPlayer))))))
    (:NewEnumerator4
      ;[0.15 0.15 0.15 0.5] Return to Stage: Take the direction that brings enemy to the Staging Area Entrance
      (return (CallFunction|GetDirectiontoControlPoint (CallFunction|GetStagingAreaControlPoint self))))))

(fn UpdateState
  (params (DeltaSeconds :type Float%20%28double-precision%29))
  (switch Utilities|FlowControl|Switch|SwitchonEEnemyBehavior (Variables|Movement|GetCurrentBehavior)
    (:NewEnumerator0
      _)
    (:NewEnumerator1
      _)
    (:NewEnumerator2
      _)
    (:NewEnumerator4
      _))
  (CallFunction|MoveTowardControlPoint DeltaSeconds))

(fn ImmediateTurn
  (Utilities|IsValid (Variables|Movement|GetPreviousControlPoint)
    (:Is%20Valid
      (Variables|Movement|SetCurrentDirection (CallFunction|GetOppositeDirection (Variables|Movement|GetCurrentDirection)))
      (LocalVariables|SetTempControlPointRef (Variables|Movement|GetTargetControlPoint))
      (Variables|Movement|SetTargetControlPoint (Variables|Movement|GetPreviousControlPoint))
      (Variables|Movement|SetPreviousControlPoint (LocalVariables|GetTempControlPointRef)))))

(fn GetControlPointClosesttoLocation
  (params (TargetLocation :type Vector))
  (bind _outactors (Actor|GetAllActorsOfClass "/Game/Blueprints/ControlPoints/BP_ControlPoint.BP_ControlPoint_C"))
  (Utilities|Array|RemoveItem _outactors (Variables|Movement|GetTargetControlPoint))
  (bind _asbp_control_point (Utilities|Casting|CastToBP_ControlPoint (.ReturnValue (Actor|FindNearestActor TargetLocation _outactors))))
  (return _asbp_control_point))

(fn GetDirectiontoControlPoint
  (params (ControlPoint :type BP%20Control%20Point%20Object%20Reference))
  ;[0.15 0.15 0.15 0.5] Hueristic: Take direction in which distance to target control point is least (Will need this to search further)
  (bind (_keypin _valuepin) (Utilities|Map|ForEachLoop(Map) (Variables|/Game/Blueprints/ControlPoints/BP_ControlPoint.BP_ControlPoint_C|GetAdjacent (Variables|Movement|GetTargetControlPoint)))
    (:then
      (if (< (Math|Vector|Distance2D(Vector) (Transformation|GetActorLocation _valuepin) (Transformation|GetActorLocation ControlPoint)) (LocalVariables|GetBestDistance))
        (LocalVariables|SetBestDirection _keypin)
        (LocalVariables|SetBestDistance (Math|Vector|Distance2D(Vector) (Transformation|GetActorLocation _valuepin) (Transformation|GetActorLocation ControlPoint)))))
    (:CompletedPin
      (return (LocalVariables|GetBestDirection)))))

(fn GetNearestControlPoint
  (bind _outactors (Actor|GetAllActorsOfClass "/Game/Blueprints/ControlPoints/BP_ControlPoint.BP_ControlPoint_C"))
  (bind _asbp_control_point (Utilities|Casting|CastToBP_ControlPoint (.ReturnValue (Actor|FindNearestActor (Transformation|GetActorLocation) _outactors))))
  (return _asbp_control_point))

(fn GetFurthestControlPointfromLocation
  (params (TargetLocation :type Vector))
  (bind _outactors (Actor|GetAllActorsOfClass "/Game/Blueprints/ControlPoints/BP_ControlPoint.BP_ControlPoint_C"))
  (Utilities|Array|RemoveItem _outactors (Variables|Movement|GetTargetControlPoint))
  (bind _asbp_control_point (Utilities|Casting|CastToBP_ControlPoint (.ReturnValue (CallFunction|FindFurthestActor TargetLocation _outactors))))
  (return _asbp_control_point))

(fn SetDamageState
  (params (NewDamageState :type EDamageState%20Enum :default "NewEnumerator0"))
  (bind _output_get (Variables|Default|SetDamageState NewDamageState))
  (switch Utilities|FlowControl|Switch|SwitchonEDamageState _output_get
    (:NewEnumerator0
      (Rendering|Material|SetMaterial (Variables|Default|GetMaskMesh) 0 (Variables|Default|GetOriginalMaterial)))
    (:NewEnumerator1
      (Rendering|Material|SetMaterial (Variables|Default|GetMaskMesh) 0 "/Game/Materials/M_Test_Blue.M_Test_Blue"))
    (:NewEnumerator2
      (Rendering|Material|SetMaterial (Variables|Default|GetMaskMesh) 0 "/Game/Materials/M_Test_Grey.M_Test_Grey"))))

(fn SetBehavior
  (params (NewBehavior :type EEnemyBehavior%20Enum :default "NewEnumerator0"))
  (bind _output_get (Variables|Movement|SetCurrentBehavior NewBehavior))
  (switch Utilities|FlowControl|Switch|SwitchonEEnemyBehavior _output_get))